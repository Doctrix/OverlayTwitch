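; CameraController handles zoom input for the city game's camera.
; Zoom in, zoom out and reset actions each call a function that writes the spring arm length on a referenced camera pawn.
; Zooming steps the length by a sensitivity value, clamped between zero and a maximum distance, while reset sets it straight to zero, the closest zoom.
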(event `InputAction|ZoomIn`
  (params (Key :type "Key Structure"))
  (:`Pressed`
    (`self.ActionInput_ZoomIn`)))

(event `InputAction|ZoomOut`
  (params (Key :type "Key Structure"))
  (:`Pressed`
    (`self.ActionInput_ZoomOut`)))

(event `InputAction|ZoomReset`
  (params (Key :type "Key Structure"))
  (:`Pressed`
    (`self.ActionInput_ZoomReset`)))

(fn `ActionInput_ZoomIn`
  (bind _springarm (`/Game/Core/CityGame/Blueprints/MainCamera.SpringArm` (`self.CameraPawnRef`)))
  (set `SpringArmComponent.TargetArmLength` (`KismetMathLibrary.FClamp` (- (`SpringArmComponent.TargetArmLength` _springarm) (`self.ZoomSensitivity`)) 0.0 (`self.MaxArmDistance`)) _springarm))

(fn `ActionInput_ZoomOut`
  (bind _springarm (`/Game/Core/CityGame/Blueprints/MainCamera.SpringArm` (`self.CameraPawnRef`)))
  (set `SpringArmComponent.TargetArmLength` (`KismetMathLibrary.FClamp` (+ (`SpringArmComponent.TargetArmLength` _springarm) (`self.ZoomSensitivity`)) 0.0 (`self.MaxArmDistance`)) _springarm))

(fn `ActionInput_ZoomReset`
  (set `SpringArmComponent.TargetArmLength` 0.0 (`/Game/Core/CityGame/Blueprints/MainCamera.SpringArm` (`self.CameraPawnRef`))))

(fn `UserConstructionScript`)