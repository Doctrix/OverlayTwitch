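; Master player controller that drives the MainCamera pawn, handling movement and zoom from player input.
; Zoom inputs step the spring arm length within limits or reset it to a default.
; Movement speed scales with arm length and can be disabled by a flag.
; Forward movement follows the camera's orientation, while sideways movement offsets along world Y and pins the height.
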(event `self.ReceiveBeginPlay`
  (`|ExecutionSequence`
    (:`then_0`
      (`self.CastReferences`))))

(event `InputAction|ZoomIn`
  (params (Key :type "Key Structure"))
  ;[1 1 1] Zoom
  (:`Pressed`
    (`self.ActionInput_ZoomIn`)))

(event `InputAction|ZoomReset`
  (params (Key :type "Key Structure"))
  ;[1 1 1] Zoom Reset
  (:`Pressed`
    (`self.ActionInput_ZoomReset`)))

(event `InputAction|ZoomOut`
  (params (Key :type "Key Structure"))
  ;[1 1 1] Zoom
  (:`Pressed`
    (`self.ActionInput_ZoomOut`)))

(event `InputAxis|MoveForward`
  (params (AxisValue :type "Float (single-precision)"))
  ;[1 1 1] Move forward
  (`self.MoveForward/Back` AxisValue))

(event `InputAxis|MoveRight`
  (params (AxisValue :type "Float (single-precision)"))
  ;[1 1 1] Move Right
  (`self.MoveRight/Left` AxisValue))

(fn `ActionInput_ZoomIn`
  (bind _springarm (`/Game/Blueprints/Pawn/MainCamera.SpringArm` (`self.CameraPawn_REF`)))
  (set `SpringArmComponent.TargetArmLength` (`KismetMathLibrary.FClamp` (- (`SpringArmComponent.TargetArmLength` _springarm) (`self.ZoomSensitivity`)) 0.0 (`self.MaxArmDistance`)) _springarm))

(fn `ActionInput_ZoomOut`
  (bind _springarm (`/Game/Blueprints/Pawn/MainCamera.SpringArm` (`self.CameraPawn_REF`)))
  (set `SpringArmComponent.TargetArmLength` (`KismetMathLibrary.FClamp` (+ (`SpringArmComponent.TargetArmLength` _springarm) (`self.ZoomSensitivity`)) 0.0 (`self.MaxArmDistance`)) _springarm))

(fn `ActionInput_ZoomReset`
  (set `SpringArmComponent.TargetArmLength` 1500.0 (`/Game/Blueprints/Pawn/MainCamera.SpringArm` (`self.CameraPawn_REF`))))

(fn `MoveForward/Back`
  (params (SpeedMultiplier :type "Float (double-precision)"))
  (if (not (`self.DisableCamNav`))
    (`self.K2_SetActorTransform` (`self.CameraPawn_REF`) (`self.MoveX` SpeedMultiplier (`self.MoveSpeedCalcul`) (`self.MoveSensitivity`) (`self.CameraPawn_REF`)) false false)
    (return)))

(fn `MoveRight/Left`
  (params (SpeedMultiplier :type "Float (double-precision)"))
  (if (not (`self.DisableCamNav`))
    (`self.K2_SetActorTransform` (`self.CameraPawn_REF`) (`KismetMathLibrary.MakeTransform` (`KismetMathLibrary.MakeVector` (.x (.location (`self.MoveY` (`self.MoveSpeedCalcul`) (`self.MoveSensitivity`) SpeedMultiplier (`self.CameraPawn_REF`)))) (.y (.location (`self.MoveY` (`self.MoveSpeedCalcul`) (`self.MoveSensitivity`) SpeedMultiplier (`self.CameraPawn_REF`)))) 100.0) (.rotation (`self.MoveY` (`self.MoveSpeedCalcul`) (`self.MoveSensitivity`) SpeedMultiplier (`self.CameraPawn_REF`))) (.scale (`self.MoveY` (`self.MoveSpeedCalcul`) (`self.MoveSensitivity`) SpeedMultiplier (`self.CameraPawn_REF`)))) false false)))

(fn `MoveSpeedCalcul`
  (returns (MoveSensitivity :type "Float (double-precision)"))
  (return (`KismetMathLibrary.FClamp` (/ (`SpringArmComponent.TargetArmLength` (`/Game/Blueprints/Pawn/MainCamera.SpringArm` (`self.CameraPawn_REF`))) 100.0) 5.0 20.0)))

(fn `UserConstructionScript`)