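; Master Game Mode Blueprint that handles startup settings and creation of the in-game HUD and main menu widgets.
; BeginPlay runs console commands for dynamic resolution and an FPS cap, then calls the HUD event.
; The HUD and AfficherLeMenu events each lazily create and cache their widget before adding it to the viewport.
; Nothing in this graph calls the menu event.
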(event `self.ReceiveBeginPlay`
  (`KismetSystemLibrary.ExecuteConsoleCommand` "r.DynamicRes.MaxConsecutiveOverbudgetGPUFrameCount" null)
  (`KismetSystemLibrary.ExecuteConsoleCommand` "t.MaxFPS 30" null)
  (`self.HUD`))

(event `HUD`
  ;[1 1 1] HUD du jeu
  (`/Engine/EditorBlueprintResources/StandardMacros.IsValid` (`self.HUD_Game`)
    (:`Is Valid`
      _)
    (:`Is Not Valid`
      (bind _returnvalue (`|CreateWidget` "/Game/Blueprints/Widgets/HUD_Game.HUD_Game_C"))
      (bind _output_get (set `self.HUD_Game` _returnvalue))))
  (`UserWidget.AddToViewport` _output_get 0))

(event `AfficherLeMenu`
  ;[1 1 1] Menu
  (`/Engine/EditorBlueprintResources/StandardMacros.IsValid` (`self.HUD_MenuMain`)
    (:`Is Valid`
      _)
    (:`Is Not Valid`
      (bind _returnvalue (`|CreateWidget` "/Game/Blueprints/Widgets/MenuMain.MenuMain_C"))
      (bind _output_get (set `self.HUD_MenuMain` _returnvalue))))
  (`UserWidget.AddToViewport` _output_get 0))

(fn `UserConstructionScript`)