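; World manager actor that runs an optional day cycle by rotating the sun.
; On BeginPlay it caches the game mode and HUD, then starts the DayCycle timeline if enabled, seeding its time from the clock hour and play rate from the minute.
; Timeline updates set sun pitch and refresh the sky material, restarting on finish.
; A separate RotationSun function spins the sun incrementally by SpeedDay and updates sky sun direction.
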(event `self.ReceiveBeginPlay`
  (bind _asgame_mode_master (cast `/Game/Blueprints/GameMode/GameMode_MASTER` (`GameplayStatics.GetGameMode`)))
  (bind _output_get (set `self.GameMode` _asgame_mode_master))
  (set `self.UI_Ref` (`/Game/Blueprints/GameMode/GameMode_MASTER.HUD_Game` _output_get))
  (if (`self.UseDayCycle`)
    (`self.StartDay`)))

(event `StartDay`
  (bind (_year _month _day _hour _minute _second) (`KismetMathLibrary.BreakDateTime` (`KismetMathLibrary.Now`)))
  (`TimelineComponent.SetPlayRate` (`self.DayCycle`) (`KismetMathLibrary.Conv_IntToDouble` _minute))
  (bind (_direction _timeofday_minute_) (`Timeline|DayCycle` :`NewTime` (`KismetMathLibrary.Conv_IntToDouble` _hour) :!via `SetNewTime`)
    (:`Update`
      (`self.K2_SetActorRotation` (`self.Sun`) (`KismetMathLibrary.ComposeRotators` (`KismetMathLibrary.MakeRotator` 0.0 _timeofday_minute_)) false)
      (`/Engine/EngineSky/BP_Sky_Sphere.RefreshMaterial` (`self.Sky`)))
    (:`Finished`
      (`self.StartDay`))))

(fn `UserConstructionScript`)